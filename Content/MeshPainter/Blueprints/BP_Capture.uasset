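; BP_Capture is a mesh-painting capture actor that renders brush hits on a target actor through an unwrap material.
; On BeginPlay it publishes capture size and location to MPC_Global, clears RT_Capture after a short delay, and creates a dynamic M_Unwrap instance.
; PaintActor temporarily swaps the mesh's first material for that instance, feeds it hit location and brush radius, triggers SceneCapture, then restores the original.
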(event `self.ReceiveBeginPlay`
  (`self.InitializeParameters`
    (:`Out`
      (bind _returnvalue (`KismetMaterialLibrary.CreateDynamicMaterialInstance` "/Game/MeshPainter/Materials/M_Unwrap.M_Unwrap"))
      (set `self.UnwrapMaterial` _returnvalue))))

(fn `PaintActor`
  (params (ActorToPaint :type "Actor Object Reference") (HitLocation :type "Vector Structure") (BrushRadius :type "Float (double-precision)"))
  (locals (MeshComponent :type "MeshComponent Object Reference") (OriginalMaterial :type "MaterialInterface Object Reference"))
  (set `local.MeshComponent` (`self.GetComponentByClass` ActorToPaint "/Script/Engine.MeshComponent"))
  (`|ExecutionSequence`
    (:`then_0`
      (set `local.OriginalMaterial` (`PrimitiveComponent.GetMaterial` (`local.MeshComponent`) 0))
      (`PrimitiveComponent.SetMaterial` (`local.MeshComponent`) 0 (`self.UnwrapMaterial`))
      (`KismetMaterialLibrary.SetVectorParameterValue` "/Game/MeshPainter/Materials/MPC_Global.MPC_Global" "UnwrapLocation" (`KismetMathLibrary.Conv_VectorToLinearColor` (`SceneComponent.K2_GetComponentLocation` (`self.SceneCapture`)))))
    (:`then_1`
      (`MaterialInstanceDynamic.SetVectorParameterValue` (`self.UnwrapMaterial`) "HitLocation" (`KismetMathLibrary.Conv_VectorToLinearColor` (`local.HitLocation`)))
      (`MaterialInstanceDynamic.SetScalarParameterValue` (`self.UnwrapMaterial`) "BrushRadius" (`local.BrushRadius`)))
    (:`then_2`
      (`SceneCaptureComponent2D.CaptureScene` (`self.SceneCapture`))
      (`PrimitiveComponent.SetMaterial` (`local.MeshComponent`) 0 (`local.OriginalMaterial`)))))

(fn `UserConstructionScript`)