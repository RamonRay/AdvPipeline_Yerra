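; BP_Player is the player Blueprint for mesh painting, letting the player shoot paint onto whatever is in view.
; On BeginPlay it waits briefly, then caches the first BP_Capture actor in the level.
; While the Shoot axis is positive, it line-traces on Visibility from the actor's location along the control rotation.
; On a hit, it passes the actor, location and fixed brush radius to BP_Capture's PaintActor and draws a debug line.
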(event `self.ReceiveBeginPlay`
  (`KismetSystemLibrary.Delay` 0.1)
  (bind _outactors (`GameplayStatics.GetAllActorsOfClass` "/Game/MeshPainter/Blueprints/BP_Capture.BP_Capture_C"))
  (bind _output (`|GetArrayItem` _outactors))
  (`/Engine/EditorBlueprintResources/StandardMacros.IsValid` _output
    (:`Is Valid`
      (set `self.CaptureActor` _output))))

(event `InputAxis|Shoot`
  (params (AxisValue :type "Float (single-precision)"))
  (if (> AxisValue 0.0)
    (`self.Shoot`)))

(fn `Shoot`
  (bind _returnvalue (`self.K2_GetActorLocation`))
  (bind _returnvalue_2 (+ _returnvalue (* (`KismetMathLibrary.GetForwardVector` (`self.GetControlRotation`)) (`self.ShootDistance`))))
  (bind (_outhit _returnvalue_3) (`KismetSystemLibrary.LineTraceSingle` _returnvalue _returnvalue_2 "TraceTypeQuery1"))
  (if _returnvalue_3
    (bind (_bblockinghit _binitialoverlap _time _distance _location _impactpoint _normal _impactnormal _physmat _hitactor) (`GameplayStatics.BreakHitResult` _outhit))
    (`/Game/MeshPainter/Blueprints/BP_Capture.PaintActor` (`self.CaptureActor`) _hitactor _location 10.0)
    (`KismetSystemLibrary.DrawDebugLine` _returnvalue _returnvalue_2)))

(fn `UserConstructionScript`)