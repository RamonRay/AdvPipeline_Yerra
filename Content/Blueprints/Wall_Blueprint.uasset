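; Wall actor that drives a proximity-triggered screen reveal effect through the Distance Material Parameter Collection.
; On BeginPlay it derives a screen size from the mesh's world scale and writes it to the collection.
; Box overlaps toggle ShowScreen, and Tick moves a reference point along Direction toward the mesh origin or out to a scaled maximum distance.
; That world position feeds the ReferencePos parameter for materials to read.
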(event `self.ReceiveBeginPlay`
  (bind _output_get (set `self.ScreenSize` (* (`KismetMathLibrary.Sqrt` (+ (+ (`KismetMathLibrary.Square` (.x (`SceneComponent.K2_GetComponentScale` (`self.StaticMeshComponent`)))) (`KismetMathLibrary.Square` (.z (`SceneComponent.K2_GetComponentScale` (`self.StaticMeshComponent`))))) (`KismetMathLibrary.Square` (* (.y (`SceneComponent.K2_GetComponentScale` (`self.StaticMeshComponent`))) 2.0)))) 50.0)))
  (`KismetMaterialLibrary.SetScalarParameterValue` "/Game/Material/Distance.Distance" "ScreenSize" _output_get))

(event `self.ReceiveTick`
  (params (DeltaSeconds :type "Float (single-precision)"))
  (bind _direction (`self.Direction`))
  (bind _referencedist (`self.ReferenceDist`))
  (bind _returnvalue (* (`self.ScreenSize`) (`self.DistMultiplier`)))
  (bind _returnvalue_2 (* (`self.SpeedPerSec`) DeltaSeconds))
  (if (`self.ShowScreen`)
    (if (> (`self.ReferenceDist`) 0.0)
      (bind _output_get (set `self.ReferenceDist` (- _referencedist _returnvalue_2)))
      (set `self.ReferencePos` (* _direction _output_get))
      (else
        (bind _output_get_2 (set `self.ReferenceDist` 0.0))
        (set `self.ReferencePos` (* _direction _output_get_2))))
    (elif (< (`self.ReferenceDist`) _returnvalue)
      (bind _output_get_3 (set `self.ReferenceDist` (+ _returnvalue_2 _referencedist)))
      (set `self.ReferencePos` (* _direction _output_get_3))
      (else
        (bind _output_get_4 (set `self.ReferenceDist` _returnvalue))
        (set `self.ReferencePos` (* _direction _output_get_4)))))
  (`KismetMaterialLibrary.SetVectorParameterValue` "/Game/Material/Distance.Distance" "ReferencePos" (`KismetMathLibrary.Conv_VectorToLinearColor` (+ (`SceneComponent.K2_GetComponentLocation` (`self.StaticMeshComponent`)) (`self.ReferencePos`)))))

(event `self.Box.OnComponentBeginOverlap`
  (params (OverlappedComponent :type "PrimitiveComponent Object Reference") (OtherActor :type "Actor Object Reference") (OtherComp :type "PrimitiveComponent Object Reference") (OtherBodyIndex :type Integer) (bFromSweep :type Boolean) (SweepResult :type "HitResult Structure (by ref)"))
  (set `self.ShowScreen` true))

(event `self.Box.OnComponentEndOverlap`
  (params (OverlappedComponent :type "PrimitiveComponent Object Reference") (OtherActor :type "Actor Object Reference") (OtherComp :type "PrimitiveComponent Object Reference") (OtherBodyIndex :type Integer))
  (set `self.ShowScreen` false))

(fn `UserConstructionScript`)