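; Spider character Blueprint that paints onto surfaces below it and drives four feet through a Control Rig.
; Before each rig update, it sets the foot controls to world-space positions supplied by four leg objects.
; While painting, a downward trace runs every tick and briefly swaps the hit mesh's material to M_Unwrap with brush location and radius.
; A scene capture records that unwrapped mesh, with the spider hidden, before the original material returns.
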(event `self.ReceiveBeginPlay`
  (`self.InitializeParameters`))

(event `self.ReceiveTick`
  (params (DeltaSeconds :type "Float (single-precision)"))
  (`SceneCaptureComponent.HideActorComponents` (`self.SceneCapture`) self true)
  (if (`self.isPainting`)
    (`self.Shoot`)))

(event `self.ControlRig.OnPreUpdateDelegate`
  (params (Component :type "ControlRigComponent Object Reference"))
  (bind _controlrig (`self.ControlRig`))
  (`ControlRigComponent.SetControlTransform` _controlrig "RightFoot" (`KismetMathLibrary.MakeTransform` (`/Game/Blueprints/BP_Leg.Foot Position` (`self.RightLeg`))) "WorldSpace")
  (`ControlRigComponent.SetControlTransform` Component "RightFoot" (`KismetMathLibrary.MakeTransform` (`/Game/Blueprints/BP_Leg.Foot Position` (`self.RightLeg`))) "WorldSpace")
  (`ControlRigComponent.SetControlTransform` _controlrig "LeftFoot" (`KismetMathLibrary.MakeTransform` (`/Game/Blueprints/BP_Leg.Foot Position` (`self.LeftLeg`))) "WorldSpace")
  (`ControlRigComponent.SetControlTransform` _controlrig "FrontFoot" (`KismetMathLibrary.MakeTransform` (`/Game/Blueprints/BP_Leg.Foot Position` (`self.FrontLeg`))) "WorldSpace")
  (`ControlRigComponent.SetControlTransform` _controlrig "BackFoot" (`KismetMathLibrary.MakeTransform` (`/Game/Blueprints/BP_Leg.Foot Position` (`self.BackLeg`))) "WorldSpace"))

(fn `PaintActor`
  (params (ActorToPaint :type "Actor Object Reference") (HitLocation :type "Vector Structure") (BrushRadius :type "Float (double-precision)") (UnwrapInstance :type "MaterialInstanceDynamic Object Reference"))
  (locals (MeshComponent :type "MeshComponent Object Reference") (OriginalMaterial :type "MaterialInterface Object Reference"))
  (bind _scenecapture (`self.SceneCapture`))
  (set `local.MeshComponent` (`self.GetComponentByClass` ActorToPaint "/Script/Engine.MeshComponent"))
  (bind _returnvalue (`KismetMaterialLibrary.CreateDynamicMaterialInstance` "/Game/MeshPainter/Materials/M_Unwrap.M_Unwrap"))
  (set `self.UnwrapMaterial` _returnvalue)
  (`|ExecutionSequence`
    (:`then_0`
      (set `local.OriginalMaterial` (`|GetArrayItem` (`MeshComponent.GetMaterials` (`local.MeshComponent`))))
      (`PrimitiveComponent.SetMaterial` (`local.MeshComponent`) 0 (`self.UnwrapMaterial`))
      (`KismetMaterialLibrary.SetVectorParameterValue` "/Game/MeshPainter/Materials/MPC_Global.MPC_Global" "UnwrapLocation" (`KismetMathLibrary.Conv_VectorToLinearColor` (`SceneComponent.K2_GetComponentLocation` (`self.SceneCapture`)))))
    (:`then_1`
      (`MaterialInstanceDynamic.SetVectorParameterValue` (`self.UnwrapMaterial`) "HitLocation" (`KismetMathLibrary.Conv_VectorToLinearColor` (`local.HitLocation`)))
      (`MaterialInstanceDynamic.SetScalarParameterValue` (`self.UnwrapMaterial`) "BrushRadius" (`local.BrushRadius`)))
    (:`then_2`
      (`SceneCaptureComponent.HideActorComponents` _scenecapture self true)
      (`SceneCaptureComponent2D.CaptureScene` _scenecapture)
      (`PrimitiveComponent.SetMaterial` (`local.MeshComponent`) 0 (`local.OriginalMaterial`)))))

(fn `Shoot`
  (bind _returnvalue (`self.K2_GetActorLocation`))
  (bind (_outhit _returnvalue_2) (`KismetSystemLibrary.LineTraceSingle` _returnvalue (+ _returnvalue (* (* (`KismetMathLibrary.GetUpVector` (struct)) -1.0) (`self.ShootDistance`))) "TraceTypeQuery1"))
  (if _returnvalue_2
    (bind (_bblockinghit _binitialoverlap _time _distance _location _impactpoint _normal _impactnormal _physmat _hitactor) (`GameplayStatics.BreakHitResult` _outhit))
    (`self.PaintActor` _hitactor _location (`self.BrushSize`))))

(fn `UserConstructionScript`
  (`ControlRigComponent.AddMappedCompleteSkeletalMesh` (`self.ControlRig`) (`self.Mesh`)))