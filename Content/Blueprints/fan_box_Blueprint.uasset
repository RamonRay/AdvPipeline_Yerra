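; Fan box Blueprint that spins its FanLeaves component continuously.
; Each Tick advances an accumulated RotateAngle by RotationSpeed plus a random amount scaled by Variance, multiplied by delta time for uneven, frame-rate-aware motion.
; The angle wraps past 360 degrees and is applied as the blades' relative pitch, with roll and yaw held at zero.
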(event `self.ReceiveTick`
  (params (DeltaSeconds :type "Float (single-precision)"))
  (`|ExecutionSequence`
    (:`then_0`
      (bind _output_get (set `self.rotateAngle` (+ (* (+ (* (`KismetMathLibrary.RandomFloat`) (`self.variance`)) (`self.rotationSpeed`)) DeltaSeconds) (`self.rotateAngle`))))
      (if (> _output_get 360.0)
        (set `self.rotateAngle` (- _output_get 360.0))))
    (:`then_1`
      (`SceneComponent.K2_SetRelativeRotation` (`self.fan_leaves`) (`KismetMathLibrary.MakeRotator` 0.0 (`self.rotateAngle`)) false false))))

(fn `UserConstructionScript`)